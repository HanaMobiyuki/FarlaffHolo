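; Player pawn that acts as a viewer control, moving and rotating a referenced Model actor.
; Axis inputs translate it along world axes; while right mouse is held, they also pitch it locally and yaw it in world space via rotator combine order.
; The mouse wheel adjusts Camera's orthographic width.
; C alternates activation between Camera and Camera1 using the QuadriView flag, without explicitly deactivating either.
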(event Input|AxisEvents|InputAxisrotate_up
  (params (AxisValue :type Float%20%28single-precision%29))
  (bind _model (Variables|Default|GetModel))
  (if (Variables|Default|Getcan_rotate)
    (Transformation|SetActorRotation _model (Math|Rotator|CombineRotators (Math|Rotator|MakeRotator 0.0 AxisValue 0.0) (Transformation|GetActorRotation _model)))))

(event Input|AxisEvents|InputAxisrotate_right
  (params (AxisValue :type Float%20%28single-precision%29))
  (bind _model (Variables|Default|GetModel))
  (if (Variables|Default|Getcan_rotate)
    (Transformation|SetActorRotation _model (Math|Rotator|CombineRotators (Transformation|GetActorRotation _model) (Math|Rotator|MakeRotator 0.0 0.0 AxisValue)))))

(event Input|AxisEvents|InputAxismove_right
  (params (AxisValue :type Float%20%28single-precision%29))
  (bind _model (Variables|Default|GetModel))
  (bind _returnvalue (Transformation|GetActorLocation _model))
  (bind (_x _y _z) (Math|Vector|BreakVector _returnvalue))
  (Transformation|SetActorLocation (Variables|Default|GetModel) (Math|Vector|MakeVector _x (+ _y AxisValue) _z) false false))

(event Input|AxisEvents|InputAxismove_front
  (params (AxisValue :type Float%20%28single-precision%29))
  (bind _model (Variables|Default|GetModel))
  (bind _returnvalue (Transformation|GetActorLocation _model))
  (bind (_x _y _z) (Math|Vector|BreakVector _returnvalue))
  (Transformation|SetActorLocation (Variables|Default|GetModel) (Math|Vector|MakeVector (+ _x AxisValue) _y _z) false false))

(event Input|AxisEvents|InputAxismove_up
  (params (AxisValue :type Float%20%28single-precision%29))
  (bind _model (Variables|Default|GetModel))
  (bind _returnvalue (Transformation|GetActorLocation _model))
  (bind (_x _y _z) (Math|Vector|BreakVector _returnvalue))
  (Transformation|SetActorLocation (Variables|Default|GetModel) (Math|Vector|MakeVector _x _y (+ _z AxisValue)) false false))

(event Input|MouseEvents|MouseWheelUp
  (params (Key :type Key%20Structure :default "AnyKey"))
  (bind _camera (Variables|Default|GetCamera))
  (:Pressed
    (Variables|/Script/Engine.CameraComponent|SetOrthoWidth _camera (- (Variables|/Script/Engine.CameraComponent|GetOrthoWidth _camera) 1e+02))))

(event Input|MouseEvents|MouseWheelDown
  (params (Key :type Key%20Structure :default "AnyKey"))
  (bind _camera (Variables|Default|GetCamera))
  (:Pressed
    (Variables|/Script/Engine.CameraComponent|SetOrthoWidth _camera (+ (Variables|/Script/Engine.CameraComponent|GetOrthoWidth _camera) 1e+02))))

(event Input|KeyboardEvents|C
  (params (Key :type Key%20Structure :default "AnyKey"))
  (:Pressed
    (if (Variables|Default|GetQuadriView)
      (Components|Activation|SetActive (Variables|Default|GetCamera1) true true)
      (Variables|Default|SetQuadriView false)
      (else
        (Components|Activation|SetActive (Variables|Default|GetCamera) true true)
        (Variables|Default|SetQuadriView true)))))

(event Input|MouseEvents|RightMouseButton
  (params (Key :type Key%20Structure :default "AnyKey"))
  (:Pressed
    (Variables|Default|Setcan_rotate true))
  (:Released
    (Variables|Default|Setcan_rotate false)))

(fn ConstructionScript)